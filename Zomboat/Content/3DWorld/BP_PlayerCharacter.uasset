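; BP_PlayerCharacter is a clickable player character with health, stamina and a record of the GroundArea it last overlapped.
; BeginPlay gathers all player characters in the level, fills stamina and caches the health widget, cast to AI_EnemyHealthWidget.
; Tick shows a flattened sphere marker while IsClicked by rescaling it, with an unfinished IsFurthestRight branch.
; TakeDamage subtracts DamageToTake from health, updates the widget and prints a debug string.
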(event `self.ReceiveBeginPlay`
  (bind _outactors (`GameplayStatics.GetAllActorsOfClass` "BP_PlayerCharacter_C"))
  (set `self.PlayerCharacterActorsInLevel` _outactors)
  (set `self.CurrentStamina` (`self.MaxStamina`))
  (bind _asai_enemy_health_widget (cast `/Game/3DWorld/AI_EnemyHealthWidget` (`WidgetComponent.GetUserWidgetObject` (`self.HealthWidget`))))
  (set `self.HealthWidgetREF` _asai_enemy_health_widget))

(event `self.ReceiveActorBeginOverlap`
  (params (OtherActor :type "Actor Object Reference"))
  (bind _asground_area (cast `/Game/3DWorld/GroundArea` OtherActor))
  (set `self.CurrentGroundArea` _asground_area))

(event `self.ReceiveTick`
  (params (DeltaSeconds :type "Float (single-precision)"))
  (if (`self.IsClicked`)
    (`SceneComponent.SetWorldScale3D` (`self.Sphere`) (4.0 4.0 0.1))
    (else
      (`SceneComponent.SetWorldScale3D` (`self.Sphere`) (0.0 0.0 0.0))))
  (if (`self.IsFurthestRight`)
    _))

(event `TakeDamage`
  (`KismetSystemLibrary.PrintString` "Damage event?")
  (bind _output_get (set `self.CurrentHealth` (- (`self.CurrentHealth`) (`self.DamageToTake`))))
  (set `/Game/3DWorld/AI_EnemyHealthWidget.Health` _output_get (`self.HealthWidgetREF`)))

(fn `UserConstructionScript`)