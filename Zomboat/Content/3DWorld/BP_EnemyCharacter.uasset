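; BP_EnemyCharacter is an enemy character that tracks its health and the ground area it stands on.
; On begin play it caches its health widget and sets health to max, and overlapping a GroundArea records it as the current area.
; A damage event subtracts DamageToTake and pushes the result to the widget.
; The enemy turn event only prints a debug message, and the cylinder click handlers are empty.
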(event `self.ReceiveBeginPlay`
  (bind _asai_enemy_health_widget (cast `/Game/3DWorld/AI_EnemyHealthWidget` (`WidgetComponent.GetUserWidgetObject` (`self.HealthWidget`))))
  (set `self.HealthWidgetREF` _asai_enemy_health_widget)
  (set `self.CurrentHealth` (`self.MaxHealth`)))

(event `self.ReceiveActorBeginOverlap`
  (params (OtherActor :type "Actor Object Reference"))
  (bind _asground_area (cast `/Game/3DWorld/GroundArea` OtherActor))
  (set `self.CurrentGroundArea` _asground_area))

(event `EnemyTurn_Event`
  (`KismetSystemLibrary.PrintString` "My turn now bitch"))

(event `TakeDamage_Event`
  (`KismetSystemLibrary.PrintString` "Damage event?")
  (bind _output_get (set `self.CurrentHealth` (- (`self.CurrentHealth`) (`self.DamageToTake`))))
  (set `/Game/3DWorld/AI_EnemyHealthWidget.Health` _output_get (`self.HealthWidgetREF`)))

(event `self.Cylinder.OnReleased`
  (params (TouchedComponent :type "PrimitiveComponent Object Reference") (ButtonReleased :type "Key Structure")))

(event `self.Cylinder.OnClicked`
  (params (TouchedComponent :type "PrimitiveComponent Object Reference") (ButtonPressed :type "Key Structure")))

(fn `UserConstructionScript`)