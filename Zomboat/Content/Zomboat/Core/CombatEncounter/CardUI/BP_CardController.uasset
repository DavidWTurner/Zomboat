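; Player controller for zombie card-combat encounters, running turns, character selection, movement and win or loss checks.
; Left-click selects a character and its card HUD; right-click AI-moves it between ground areas sorted by spawn distance, gated by enemies and in-combat stamina, or collects items as cards.
; Turn changes reset players or trigger enemies.
; Deaths clear combat areas, show rewards or tutorial messages, or open GameOver.
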(event `Key|F`
  (params (Key :type "Key Structure")))

(event `self.ReceiveTick`
  (params (DeltaSeconds :type "Float (single-precision)")))

(event `self.ReceiveBeginPlay`
  (bind _returnvalue (`|CreateWidget` "/Game/Zomboat/Core/CombatEncounter/CardUI/W_MainHUD.W_MainHUD_C"))
  (bind _output_get (set `self.MainHUDWidget` _returnvalue))
  (`UserWidget.AddToViewport` _output_get -1)
  ;[1 1 1] Delay to await world generation
  (`KismetSystemLibrary.Delay` 0.5)
  ;[1 1 1] UI and mouse input
  (`WidgetBlueprintLibrary.SetInputMode_GameAndUIEx` self null "LockAlways" false)
  (set `self.bShowMouseCursor` true)
  ;[1 1 1] Finding and sorting ground areas
  (bind _outactors (`GameplayStatics.GetAllActorsOfClass` "/Game/Zomboat/Core/CombatEncounter/3DWorld/GroundArea.GroundArea_C"))
  (bind _output_get_2 (set `self.GroundAreasInLevel` _outactors))
  ;;[1 1 1] This function sorts the ground area refs in to left right order
  (bind _sorted_by_distance (`self.SortArraybyDistanceFromPlayerSpawn` _output_get_2))
  (set `self.GroundAreasInLevel` _sorted_by_distance)
  ;[1 1 1] Finding and storing enemies
  (bind _arrayofaliveenemies (`self.FindAliveEnemiesInLevel`))
  (set `self.EnemyCharactersInLevel` _arrayofaliveenemies)
  ;[1 1 1] Finding and storing players
  (bind _arrayofaliveenemies_2 (`self.FindAlivePlayerCharactersInLevel`))
  (bind _output_get_3 (set `self.PlayerCharacterActorsInLevel` _arrayofaliveenemies_2))
  ;[1 1 1] Make the HUD for each character and attach it to them
  (`self.Create and Attach Player HUDs` _output_get_3)
  ;[1 1 1] Ugly move player characters to their starting positions. To be replaced once the player can set the prefered default positions for each character
  (for (_array_element _array_index) (`self.PlayerCharacterActorsInLevel`)
    (bind _output_get_4 (set `self.CurrentActorToMove` _array_element))
    (switch `int` _array_index
      (:`0`
        (bind (_distance _returnvalue_2) (`GameplayStatics.FindNearestActor` (`self.K2_GetActorLocation` _output_get_4) (`self.GroundAreasInLevel`)))
        (bind (_origin _boxextent) (`self.GetActorBounds` _returnvalue_2 false false))
        (`AITask_MoveTo.AIMoveTo` (`AIBlueprintHelperLibrary.GetAIController` (`self.CurrentActorToMove`)) _origin null 0.5))
      (:`1`
        (bind _returnvalue_3 (`self.K2_GetActorLocation` _returnvalue_2))
        (bind _returnvalue_4 (/ (* (.x _boxextent) 2.0) 3.0))
        (`AITask_MoveTo.AIMoveTo` (`AIBlueprintHelperLibrary.GetAIController` (`self.CurrentActorToMove`)) (- _returnvalue_3 (`KismetMathLibrary.MakeVector` _returnvalue_4)) null 0.5))
      (:`2`
        (`AITask_MoveTo.AIMoveTo` (`AIBlueprintHelperLibrary.GetAIController` (`self.CurrentActorToMove`)) (+ _returnvalue_3 (`KismetMathLibrary.MakeVector` _returnvalue_4)) null 0.5)))))

(event `ChangeTurn`
  (bind _arrayofaliveenemies (`self.FindAliveEnemiesInLevel`))
  (set `self.EnemyCharactersInLevel` _arrayofaliveenemies)
  (bind _arrayofaliveenemies_2 (`self.FindAlivePlayerCharactersInLevel`))
  (set `self.PlayerCharacterActorsInLevel` _arrayofaliveenemies_2)
  (switch `/Game/Zomboat/Core/CombatEncounter/3DWorld/TurnEnum` (`self.CurrentTurn`)
    (:`NewEnumerator0`
      (`KismetSystemLibrary.PrintString` "PlayerTurn")
      (for _array_element (`self.PlayerCharacterActorsInLevel`)
        ;[1 1 1] Show End turn button
        (set `Widget.Visibility` "Visible" (`/Game/Zomboat/Core/CombatEncounter/CardUI/W_CardHUD.EndTurnButton` (`/Game/Zomboat/Core/CombatEncounter/3DWorld/BP_PlayerCharacter.LinkedCardHUD` _array_element)))
        ;[1 1 1] Fill stamina
        (`/Game/Zomboat/Core/CombatEncounter/3DWorld/BP_PlayerCharacter.ResetStamina` _array_element)
        ;[1 1 1] Reset block to Zero
        (`/Game/Zomboat/Core/CombatEncounter/3DWorld/BP_PlayerCharacter.ModifyBlock` _array_element (- 0.0 (`/Game/Zomboat/Core/CombatEncounter/3DWorld/BP_PlayerCharacter.CurrentBlock` _array_element)))
        ;[1 1 1] If in combat, refill hand
        (if (`/Game/Zomboat/Core/CombatEncounter/3DWorld/BP_PlayerCharacter.CharInCombat?` _array_element)
          (`/Game/Zomboat/Core/CombatEncounter/CardUI/W_CardHand.FillHandBPI` (`/Game/Zomboat/Core/CombatEncounter/CardUI/W_CardHUD.W_CardHand` (`/Game/Zomboat/Core/CombatEncounter/3DWorld/BP_PlayerCharacter.LinkedCardHUD` _array_element))))))
    (:`NewEnumerator1`
      (`KismetSystemLibrary.PrintString` "EnemyTurn")
      (for _array_element_2 (`self.PlayerCharacterActorsInLevel`)
        (if (`/Game/Zomboat/Core/CombatEncounter/3DWorld/BP_PlayerCharacter.CardsInHand` _array_element_2)
          ;[1 1 1] Hide end turn button
          (set `Widget.Visibility` "Hidden" (`/Game/Zomboat/Core/CombatEncounter/CardUI/W_CardHUD.EndTurnButton` (`/Game/Zomboat/Core/CombatEncounter/3DWorld/BP_PlayerCharacter.LinkedCardHUD` _array_element_2)))
          ;[1 1 1] Empty player hands
          (`/Game/Zomboat/Core/CombatEncounter/CardUI/W_CardHand.EmptyHand` (`/Game/Zomboat/Core/CombatEncounter/CardUI/W_CardHUD.W_CardHand` (`/Game/Zomboat/Core/CombatEncounter/3DWorld/BP_PlayerCharacter.LinkedCardHUD` _array_element_2)))
          (set `/Game/Zomboat/Core/CombatEncounter/3DWorld/BP_PlayerCharacter.CardsInHand` false _array_element_2)))
      (for _array_element_3 (`self.EnemyCharactersInLevel`)
        ;[1 1 1] Trigger enemy turn behaviour
        (`/Game/Zomboat/Core/CombatEncounter/3DWorld/BP_EnemyCharacter.EnemyTurn_Event` _array_element_3))
      ;[1 1 1] Delay to make it seem like enemy turn takes a mo
      (`KismetSystemLibrary.Delay` 1.0)
      (`self.SwitchTurn`)
      (`self.ChangeTurn`))))

(event `Key|LeftMouseButton`
  (params (Key :type "Key Structure"))
  (bind (_hitresult _returnvalue) (`self.GetHitResultUnderCursorByChannel` "TraceTypeQuery1"))
  (bind _castclickedactor (`self.CastClickedActor`))
  (bind (_bblockinghit _binitialoverlap _time _distance _location _impactpoint _normal _impactnormal _physmat _hitactor) (`GameplayStatics.BreakHitResult` _hitresult))
  (:`Pressed`
    (switch `/Game/Zomboat/Core/CombatEncounter/3DWorld/TurnEnum` (`self.CurrentTurn`)
      (:`NewEnumerator0`
        (if _returnvalue
          (if (`KismetSystemLibrary.IsValid` _hitactor)
            (if (`self.ActorHasTag` _hitactor "PlayerCharacter")
              (bind _output_get (set `self.ClickedActor` _hitactor))
              (bind _asbp_player_character (cast `/Game/Zomboat/Core/CombatEncounter/3DWorld/BP_PlayerCharacter` _output_get))
              (if (`/Game/Zomboat/Core/CombatEncounter/3DWorld/BP_PlayerCharacter.IsDead` _asbp_player_character)
                (`KismetSystemLibrary.PrintString` "They're dead, Son")
                (else
                  (set `self.CastClickedActor` _asbp_player_character)
                  (for _array_element (`self.PlayerCharacterActorsInLevel`)
                    (`self.HideUIForPlayer` _array_element)
                    (`PrimitiveComponent.SetRenderCustomDepth` (`Character.Mesh` _array_element) false))
                  (`self.ShowUIForPlayer` _castclickedactor)
                  (`PrimitiveComponent.SetRenderCustomDepth` (`Character.Mesh` _castclickedactor) true)
                  (if (`/Game/Zomboat/Core/CombatEncounter/3DWorld/BP_PlayerCharacter.CardsInHand` (`self.CastClickedActor`))
                    _
                    (elif (`/Game/Zomboat/Core/CombatEncounter/3DWorld/BP_PlayerCharacter.CharInCombat?` (`self.CastClickedActor`))
                      ;[1 1 1] STUPID DELAY BUT AT LEAST IT WORKS
                      (`KismetSystemLibrary.Delay` 0.1)
                      (message `/Game/Zomboat/Core/CombatEncounter/CardUI/BPI_FillHand.FillHandBPI` (`/Game/Zomboat/Core/CombatEncounter/CardUI/W_CardHUD.W_CardHand` (`/Game/Zomboat/Core/CombatEncounter/3DWorld/BP_PlayerCharacter.LinkedCardHUD` (`self.CastClickedActor`))))
                      (set `/Game/Zomboat/Core/CombatEncounter/3DWorld/BP_PlayerCharacter.CardsInHand` true (`self.CastClickedActor`))))))
              (elif (`self.ActorHasTag` _hitactor "Enemy")
                _))))))))

(event `Key|RightMouseButton`
  (params (Key :type "Key Structure"))
  (bind (_hitresult _returnvalue) (`self.GetHitResultUnderCursorByChannel` "TraceTypeQuery1"))
  (bind _returnvalue_2 (`GameplayStatics.GetPlayerController` 0))
  (bind _castclickedactor (`self.CastClickedActor`))
  (bind (_bblockinghit _binitialoverlap _time _distance _location _impactpoint _normal _impactnormal _physmat _hitactor) (`GameplayStatics.BreakHitResult` _hitresult))
  (bind (_grounditeminfo_itemname _grounditeminfo_displayname _grounditeminfo_linkedcards) (break `/Game/Zomboat/Core/CombatEncounter/CardUI/S_GroundItems` (`/Game/Zomboat/Core/CombatEncounter/3DWorld/BP_GroundItem.GroundItemInfo` (`self.CastGroundItem`))))
  (bind (_characterinfo_charactername _characterinfo_skeletalmesh _characterinfo_animationblueprint _characterinfo_currenthealth _characterinfo_currentstamina _characterinfo_righthanditem _characterinfo_lefthanditem _characterinfo_headitem _characterinfo_bodyitem _characterinfo_armsitem _characterinfo_legsitem _characterinfo_maxhealth _characterinfo_maxstamina _characterinfo_characternumber) (break `/Game/Zomboat/Core/CombatEncounter/3DWorld/S_Characters` (`/Game/Zomboat/Core/CombatEncounter/3DWorld/BP_PlayerCharacter.CharacterInfo` _castclickedactor)))
  (bind _returnvalue_3 (`self.ActorHasTag` _hitactor "GroundArea"))
  (:`Pressed`
    (switch `/Game/Zomboat/Core/CombatEncounter/3DWorld/TurnEnum` (`self.CurrentTurn`)
      (:`NewEnumerator0`
        (bind _asbp_player_character (cast `/Game/Zomboat/Core/CombatEncounter/3DWorld/BP_PlayerCharacter` (`self.ClickedActor`)))
        (set `self.CastClickedActor` _asbp_player_character)
        (if _returnvalue
          (set `self.RightMouseClickLocation` _location)
          (if _returnvalue_3
            (set `self.IsGroundArea` _returnvalue_3)
            (bind _output_get (set `self.ClickedGround` _hitactor))
            (bind _asground_area (cast `/Game/Zomboat/Core/CombatEncounter/3DWorld/GroundArea` _output_get)
              (:`then`
                _)
              (:`CastFailed`
                _))
            (set `self.CastClickedGroundArea` _asground_area)
            (if (== (`/Game/Zomboat/Core/CombatEncounter/3DWorld/BP_PlayerCharacter.CurrentGroundArea` (`self.CastClickedActor`)) (`self.ClickedGround`))
              (if (`self.IsGroundArea`)
                (`AITask_MoveTo.AIMoveTo` (`AIBlueprintHelperLibrary.GetAIController` (`self.CastClickedActor`)) (`self.RightMouseClickLocation`) null 0.5))
              (elif (`self.EnemiesInTheWay?`)
                _
                (elif (`/Game/Zomboat/Core/CombatEncounter/3DWorld/BP_PlayerCharacter.CharInCombat?` _castclickedactor)
                  (bind (_returnvalue_4 _staminacosttocompletemove) (`self.Is Move in Stamina Range?`))
                  (if _returnvalue_4
                    (`/Game/Zomboat/Core/CombatEncounter/3DWorld/BP_PlayerCharacter.Modify Stamina` (`self.CastClickedActor`) (- 0.0 _staminacosttocompletemove))
                    (`self.MoveActorToClickedGround` _characterinfo_characternumber :!label _label
                      (:`OutputPin`
                        (`self.EnableInput` _returnvalue_2 _returnvalue_2)
                        (if (`/Game/Zomboat/Core/CombatEncounter/3DWorld/GroundArea.IsCombatArea` (`self.CastClickedGroundArea`))
                          (set `/Game/Zomboat/Core/CombatEncounter/3DWorld/BP_PlayerCharacter.CharInCombat?` true (`self.CastClickedActor`))
                          (bind _arrayofaliveenemies (`self.FindAliveEnemiesInLevel`))
                          (bind _output_get_2 (set `self.EnemyCharactersInLevel` _arrayofaliveenemies))
                          (for _array_element _output_get_2
                            (`/Game/Zomboat/Core/CombatEncounter/3DWorld/BP_EnemyCharacter.PlayerCharacterHasMoved` _array_element)
                            (if (< (`self.GetDistanceTo` _array_element (`self.CastClickedGroundArea`)) 1000.0)
                              (set `/Game/Zomboat/Core/CombatEncounter/3DWorld/BP_EnemyCharacter.InCombat` true _array_element))))))
                    (else
                      ;[1 1 1] Not enough Stamina
                      (`/Game/Zomboat/Core/CombatEncounter/3DWorld/BP_PlayerCharacter.NotEnoughStamina` (`self.CastClickedActor`))))
                  (else
                    (goto _label)))))
            (elif (`self.ActorHasTag` _hitactor "GroundItem")
              (bind _asbp_ground_item (cast `/Game/Zomboat/Core/CombatEncounter/3DWorld/BP_GroundItem` _hitactor))
              (set `self.CastGroundItem` _asbp_ground_item)
              (if (== (`/Game/Zomboat/Core/CombatEncounter/3DWorld/BP_PlayerCharacter.CurrentGroundArea` (`self.CastClickedActor`)) (`/Game/Zomboat/Core/CombatEncounter/3DWorld/BP_GroundItem.CurrentGroundArea` (`self.CastGroundItem`)))
                (`AITask_MoveTo.AIMoveTo` (`AIBlueprintHelperLibrary.GetAIController` (`self.CastClickedActor`)) (`self.K2_GetActorLocation` (`self.CastGroundItem`)) null 0.5
                  (:`OnMoveFinished`
                    (for _array_element_2 _grounditeminfo_linkedcards
                      (bind _returnvalue_5 (`|GetDataTableRow` "/Game/Zomboat/Core/CombatEncounter/CardUI/DT_Cards.DT_Cards" (`KismetStringLibrary.Conv_StringToName` (`|GetEnumeratorNameAsString` _array_element_2)))
                        (:`then`
                          (message `/Game/Zomboat/Core/CombatEncounter/CardUI/BPI_AddCard.AddCard` (`/Game/Zomboat/Core/CombatEncounter/CardUI/W_CardHUD.W_CardHand` (`/Game/Zomboat/Core/CombatEncounter/3DWorld/BP_PlayerCharacter.LinkedCardHUD` (`self.CastClickedActor`))) _returnvalue_5))))
                    (`self.K2_DestroyActor` (`self.CastGroundItem`))))))))))))

(event `PlayerCharacterIsDying`
  (`KismetSystemLibrary.Delay` 0.5)
  (bind _arrayofaliveenemies (`self.FindAlivePlayerCharactersInLevel`))
  (set `self.PlayerCharacterActorsInLevel` _arrayofaliveenemies)
  (if (< (`KismetArrayLibrary.Array_Length` (`self.PlayerCharacterActorsInLevel`)) 1)
    (`GameplayStatics.OpenLevel` "GameOver")))

(event `ZombieDeath`
  (params (EnemyCharacter :type "/Game/Zomboat/Core/CombatEncounter/3DWorld/BP_EnemyCharacter Object Reference"))
  (bind _tutorialwidget (`self.TutorialWidget`))
  (bind _enemycharactersinlevel (`self.EnemyCharactersInLevel`))
  (set `self.CurrentlyDyingZombieLocation` (`self.K2_GetActorLocation` EnemyCharacter))
  (set `self.CurrentlyDyingZombieGroundArea` (`/Game/Zomboat/Core/CombatEncounter/3DWorld/BP_EnemyCharacter.CurrentGroundArea` EnemyCharacter))
  (`KismetSystemLibrary.Delay` 0.2)
  (bind _arrayofaliveenemies (`self.FindAliveEnemiesInLevel`))
  (set `self.EnemyCharactersInLevel` _arrayofaliveenemies)
  (if (== (`KismetArrayLibrary.Array_Length` (`self.EnemyCharactersInLevel`)) 0)
    ;[1 1 1] If it's inside1 then show the rewards screen
    (bind _returnvalue (`GameplayStatics.GetActorOfClass` "/Game/Zomboat/Core/CombatEncounter/3DWorld/BP_EndTriggerZone_Inside.BP_EndTriggerZone_Inside_C"))
    (`/Engine/EditorBlueprintResources/StandardMacros.IsValid` _returnvalue
      (:`Is Valid`
        (bind _returnvalue_2 (`|CreateWidget` "/Game/Zomboat/Developers/Phil/RewardsScreen_BP.RewardsScreen_BP_C"))
        (`UserWidget.AddToViewport` _returnvalue_2 0))
      (:`Is Not Valid`
        ;[1 1 1] Tutorial: Show the killed all zombies message
        (bind _foundwidgets (`WidgetBlueprintLibrary.GetAllWidgetsOfClass` "/Game/Zomboat/Core/Tutorial/W_Tutorial.W_Tutorial_C"))
        (for _array_element _foundwidgets
          (set `self.TutorialWidget` _array_element))
        (`/Engine/EditorBlueprintResources/StandardMacros.IsValid` _tutorialwidget
          (:`Is Valid`
            (`/Game/Zomboat/Core/Tutorial/W_Tutorial.AllEnemiesDead` _tutorialwidget)
            (for _array_element_2 (`self.PlayerCharacterActorsInLevel`)
              (for _index (range (+ (`/Game/Zomboat/Core/CombatEncounter/3DWorld/GroundArea.PositionInArray` (`self.CurrentlyDyingZombieGroundArea`)) 1))
                (bind _output (`|GetArrayItem` (`self.GroundAreasInLevel`) _index))
                (set `/Game/Zomboat/Core/CombatEncounter/3DWorld/GroundArea.IsCombatArea` false _output)
                (set `/Game/Zomboat/Core/CombatEncounter/3DWorld/GroundArea.IsDamageArea` false _output)
                (`/Game/Zomboat/Core/CombatEncounter/3DWorld/GroundArea.ChangeColour` _output))))
          (:`Is Not Valid`
            ;[1 1 1] Regular play all enemies dead behaviour
            (for _array_element_3 (`self.GroundAreasInLevel`)
              (set `/Game/Zomboat/Core/CombatEncounter/3DWorld/GroundArea.IsCombatArea` false _array_element_3)
              (set `/Game/Zomboat/Core/CombatEncounter/3DWorld/GroundArea.IsDamageArea` false _array_element_3)
              (`/Game/Zomboat/Core/CombatEncounter/3DWorld/GroundArea.ChangeColour` _array_element_3))))))
    (elif (== (`KismetArrayLibrary.Array_Length` _enemycharactersinlevel) 0)
      (for _index_2 (range (+ (`/Game/Zomboat/Core/CombatEncounter/3DWorld/GroundArea.PositionInArray` (`self.CurrentlyDyingZombieGroundArea`)) 1)) :!label _label_2
        (bind _output_2 (`|GetArrayItem` (`self.GroundAreasInLevel`) _index_2))
        (set `/Game/Zomboat/Core/CombatEncounter/3DWorld/GroundArea.IsCombatArea` false _output_2)
        (set `/Game/Zomboat/Core/CombatEncounter/3DWorld/GroundArea.IsDamageArea` false _output_2)
        (`/Game/Zomboat/Core/CombatEncounter/3DWorld/GroundArea.ChangeColour` _output_2))
      (elif (> (`GameplayStatics.FindNearestActor` (`self.CurrentlyDyingZombieLocation`) _enemycharactersinlevel) 1500.0)
        (goto _label_2)))))

(fn `Create and Attach Player HUDs`
  (params (`Player Char Array` :type "Array of /Game/Zomboat/Core/CombatEncounter/3DWorld/BP_PlayerCharacter Object Reference"))
  (bind _characterhud (`self.CharacterHUD`))
  ;[1 1 1] Adding card HUD to each player character in level
  (for _array_element `Player Char Array`
    (bind _returnvalue (`|CreateWidget` "/Game/Zomboat/Core/CombatEncounter/CardUI/W_CardHUD.W_CardHUD_C" self _array_element))
    (bind _output_get (set `self.CharacterHUD` _returnvalue))
    (`KismetArrayLibrary.Array_Add` (`self.HUDWidgets`) _output_get)
    (`UserWidget.AddToViewport` _characterhud 0)
    ;;[1 1 1] Handle mouse input
    (`WidgetBlueprintLibrary.SetInputMode_GameAndUIEx` self _characterhud "DoNotLock" false)
    (set `self.bShowMouseCursor` true)
    (`Widget.SetVisibility` (`self.CharacterHUD`) "Hidden"))
  (return))

(fn `EnemiesInTheWay?`
  (returns (`EnemiesStillThere?` :type Boolean))
  (locals (LocalEnemiesPresent :type Boolean))
  (bind _castclickedgroundarea (`self.CastClickedGroundArea`))
  (if (or (`/Game/Zomboat/Core/CombatEncounter/3DWorld/GroundArea.IsDamageArea` _castclickedgroundarea) (`/Game/Zomboat/Core/CombatEncounter/3DWorld/GroundArea.IsCombatArea` _castclickedgroundarea))
    (for _index (range (`/Game/Zomboat/Core/CombatEncounter/3DWorld/GroundArea.PositionInArray` (`/Game/Zomboat/Core/CombatEncounter/3DWorld/BP_PlayerCharacter.CurrentGroundArea` (`self.CastClickedActor`))) (+ (- (`/Game/Zomboat/Core/CombatEncounter/3DWorld/GroundArea.PositionInArray` (`self.CastClickedGroundArea`)) 2) 1))
      (bind _output (`|GetArrayItem` (`self.GroundAreasInLevel`) _index))
      (if (or (`/Game/Zomboat/Core/CombatEncounter/3DWorld/GroundArea.IsDamageArea` _output) (`/Game/Zomboat/Core/CombatEncounter/3DWorld/GroundArea.IsCombatArea` _output))
        (set `local.LocalEnemiesPresent` true)
        (break)))
    (return (`local.LocalEnemiesPresent`))
    (else
      (for _index_2 (range (`/Game/Zomboat/Core/CombatEncounter/3DWorld/GroundArea.PositionInArray` (`/Game/Zomboat/Core/CombatEncounter/3DWorld/BP_PlayerCharacter.CurrentGroundArea` (`self.CastClickedActor`))) (`/Game/Zomboat/Core/CombatEncounter/3DWorld/GroundArea.PositionInArray` (`self.CastClickedGroundArea`)))
        (bind _output_2 (`|GetArrayItem` (`self.GroundAreasInLevel`) _index_2))
        (if (or (`/Game/Zomboat/Core/CombatEncounter/3DWorld/GroundArea.IsDamageArea` _output_2) (`/Game/Zomboat/Core/CombatEncounter/3DWorld/GroundArea.IsCombatArea` _output_2))
          (set `local.LocalEnemiesPresent` true)
          (break)))
      (return (`local.LocalEnemiesPresent`)))))

(fn `FindAliveEnemiesInLevel`
  (returns (ArrayOfAliveEnemies :type "Array of /Game/Zomboat/Core/CombatEncounter/3DWorld/BP_EnemyCharacter Object Reference"))
  (locals (LocalAliveEnemiesInLevel :type "Array of /Game/Zomboat/Core/CombatEncounter/3DWorld/BP_EnemyCharacter Object Reference"))
  ;[1 1 1] Finding and storing enemies
  (bind _outactors (`GameplayStatics.GetAllActorsOfClass` "/Game/Zomboat/Core/CombatEncounter/3DWorld/BP_EnemyCharacter.BP_EnemyCharacter_C"))
  (for _array_element _outactors
    (if (not (`/Game/Zomboat/Core/CombatEncounter/3DWorld/BP_EnemyCharacter.IsDead` _array_element))
      (`KismetArrayLibrary.Array_Add` (`local.LocalAliveEnemiesInLevel`) _array_element)))
  (return (`local.LocalAliveEnemiesInLevel`)))

(fn `FindAlivePlayerCharactersInLevel`
  (returns (ArrayOfAliveEnemies :type "Array of /Game/Zomboat/Core/CombatEncounter/3DWorld/BP_PlayerCharacter Object Reference"))
  (locals (LocalAlivePlayersInLevel :type "Array of /Game/Zomboat/Core/CombatEncounter/3DWorld/BP_PlayerCharacter Object Reference"))
  ;[1 1 1] Finding and storing enemies
  (bind _outactors (`GameplayStatics.GetAllActorsOfClass` "/Game/Zomboat/Core/CombatEncounter/3DWorld/BP_PlayerCharacter.BP_PlayerCharacter_C"))
  (for _array_element _outactors
    (if (not (`/Game/Zomboat/Core/CombatEncounter/3DWorld/BP_PlayerCharacter.IsDead` _array_element))
      (`KismetArrayLibrary.Array_Add` (`local.LocalAlivePlayersInLevel`) _array_element)))
  (return (`local.LocalAlivePlayersInLevel`)))

(fn `GetActorUnderCursor`
  (returns (HitResult :type "HitResult Structure") (`HitAnything?` :type Boolean))
  (bind (_hitresult _returnvalue) (`self.GetHitResultUnderCursorByChannel` "TraceTypeQuery1"))
  (if _returnvalue
    (return _hitresult _returnvalue)
    (else
      (`KismetSystemLibrary.PrintString` "Nothing here boss"))))

(fn `HideUIForPlayer`
  (params (Actor :type "/Game/Zomboat/Core/CombatEncounter/3DWorld/BP_PlayerCharacter Object Reference"))
  (locals (LocalLoopActor :type "/Game/Zomboat/Core/CombatEncounter/3DWorld/BP_PlayerCharacter Object Reference"))
  (bind _localloopactor (`local.LocalLoopActor`))
  (set `local.LocalLoopActor` Actor)
  (if (`/Game/Zomboat/Core/CombatEncounter/3DWorld/BP_PlayerCharacter.IsClicked` (`local.LocalLoopActor`))
    (set `/Game/Zomboat/Core/CombatEncounter/3DWorld/BP_PlayerCharacter.IsClicked` false _localloopactor)
    (`Widget.SetVisibility` (`|GetArrayItem` (`self.HUDWidgets`) (`KismetArrayLibrary.Array_Find` (`self.PlayerCharacterActorsInLevel`) _localloopactor)) "Hidden")))

(fn `Is Move in Stamina Range?`
  (returns (ReturnValue :type Boolean) (StaminaCostToCompleteMove :type "Float (double-precision)"))
  (bind _groundareasinlevel (`self.GroundAreasInLevel`))
  (bind _returnvalue (`KismetMathLibrary.Abs` (- (`KismetArrayLibrary.Array_Find` _groundareasinlevel (`self.CastClickedGroundArea`)) (`KismetArrayLibrary.Array_Find` _groundareasinlevel (`/Game/Zomboat/Core/CombatEncounter/3DWorld/BP_PlayerCharacter.CurrentGroundArea` (`self.CastClickedActor`))))))
  (if (`self.ActorHasTag` (`self.ClickedGround`) "Finish")
    ;[1 1 1] If it's the finish the distance and stamina cost don't matter
    (return true 0.0)
    (else
      (return (>= (`/Game/Zomboat/Core/CombatEncounter/3DWorld/BP_PlayerCharacter.CurrentStamina` (`self.CastClickedActor`)) _returnvalue) _returnvalue))))

(fn `ShowUIForPlayer`
  (params (Actor :type "/Game/Zomboat/Core/CombatEncounter/3DWorld/BP_PlayerCharacter Object Reference"))
  (set `/Game/Zomboat/Core/CombatEncounter/3DWorld/BP_PlayerCharacter.IsClicked` true Actor)
  (bind _output_get (set `/Game/Zomboat/Core/CombatEncounter/3DWorld/BP_PlayerCharacter.LinkedCardHUD` (`|GetArrayItem` (`self.HUDWidgets`) (`KismetArrayLibrary.Array_Find` (`self.PlayerCharacterActorsInLevel`) (`self.CastClickedActor`))) (`self.CastClickedActor`)))
  (`Widget.SetVisibility` _output_get "SelfHitTestInvisible")
  (return))

(fn `SortArraybyDistanceFromPlayerSpawn`
  (params (Array :type "Array of /Game/Zomboat/Core/CombatEncounter/3DWorld/GroundArea Object Reference"))
  (returns (`Sorted By Distance` :type "Array of /Game/Zomboat/Core/CombatEncounter/3DWorld/GroundArea Object Reference"))
  (locals (WorkingArray :type "Array of /Game/Zomboat/Core/CombatEncounter/3DWorld/GroundArea Object Reference") (CurrentGroundArea :type "/Game/Zomboat/Core/CombatEncounter/3DWorld/GroundArea Object Reference") (CurrentDistance :type "Float (single-precision)" :default 0.0) (InsertIndex :type Integer :default 0) (SortedArray :type "Array of /Game/Zomboat/Core/CombatEncounter/3DWorld/GroundArea Object Reference"))
  (bind _output_get (set `local.WorkingArray` Array))
  (for _array_element _output_get
    (bind _output_get_2 (set `local.CurrentGroundArea` _array_element))
    ;[1 1 1] Get compartive value
    (bind _returnvalue (`GameplayStatics.GetActorOfClass` "/Game/Zomboat/Core/CombatEncounter/3DWorld/BP_PlayerSpawner.BP_PlayerSpawner_C"))
    (set `local.CurrentDistance` (`self.GetDistanceTo` _output_get_2 _returnvalue))
    ;[1 1 1] Add to end by default
    (set `local.InsertIndex` (`KismetArrayLibrary.Array_Length` (`local.SortedArray`)))
    ;[1 1 1] Loop backward through already sorted list. If a new actor is closer to the player, move it down the list
    (bind (_arrayindex _arrayelement) (`/Engine/EditorBlueprintResources/StandardMacros.ReverseForEachLoop` (`local.SortedArray`))
      (:`LoopBody`
        (bind _returnvalue_2 (`GameplayStatics.GetActorOfClass` "/Game/Zomboat/Core/CombatEncounter/3DWorld/BP_PlayerSpawner.BP_PlayerSpawner_C"))
        (if (> (`self.GetDistanceTo` _arrayelement _returnvalue_2) (`local.CurrentDistance`))
          (set `local.InsertIndex` _arrayindex)))
      (:`Completed`
        (`KismetArrayLibrary.Array_Insert` (`local.SortedArray`) (`local.CurrentGroundArea`) (`local.InsertIndex`)))))
  (return (`local.SortedArray`)))

(fn `SwitchTurn`
  (if (`|EnumEquality` (`self.CurrentTurn`) "NewEnumerator0")
    (set `self.CurrentTurn` "NewEnumerator1")
    (else
      (set `self.CurrentTurn` "NewEnumerator0"))))

(fn `UserConstructionScript`)