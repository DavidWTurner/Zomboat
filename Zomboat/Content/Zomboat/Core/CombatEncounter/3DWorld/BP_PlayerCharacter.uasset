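; Player character pawn for card-driven combat encounters, built from a character info struct that supplies mesh, animation, stamina and socket-attached equipment, with a tutorial override from the game instance.
; Damage drains block before health; health, block and stamina changes are pushed to the linked card HUD and per-slot main HUD.
; Short timed flags signal animation states, ground-area overlaps flag combat, and Tick reports death to BP_CardController.
; A function writes current health back to the game instance.
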(event `self.ReceiveBeginPlay`
  (bind (_characterinfo_charactername _characterinfo_skeletalmesh _characterinfo_animationblueprint _characterinfo_currenthealth _characterinfo_currentstamina _characterinfo_righthanditem _characterinfo_lefthanditem _characterinfo_headitem _characterinfo_bodyitem _characterinfo_armsitem _characterinfo_legsitem _characterinfo_maxhealth _characterinfo_maxstamina) (break `/Game/Zomboat/Core/CombatEncounter/3DWorld/S_Characters` (`self.CharacterInfo`)))
  (bind _mesh (`self.Mesh`))
  (bind _asbp_card_controller (cast `/Game/Zomboat/Core/CombatEncounter/CardUI/BP_CardController` (`GameplayStatics.GetPlayerController` 0)))
  (set `self.CastCardController` _asbp_card_controller)
  (`self.GetTutorialCharDetails`)
  ;[1 1 1] Get and sort ground areas
  (bind _outactors (`GameplayStatics.GetAllActorsOfClass` "/Game/Zomboat/Core/CombatEncounter/3DWorld/GroundArea.GroundArea_C"))
  (bind _output_get (set `self.GroundAreas` _outactors))
  (bind _asbp_card_controller_2 (cast `/Game/Zomboat/Core/CombatEncounter/CardUI/BP_CardController` (`GameplayStatics.GetPlayerController` 0)))
  (bind _sorted_by_distance (`/Game/Zomboat/Core/CombatEncounter/CardUI/BP_CardController.SortArraybyDistanceFromPlayerSpawn` _asbp_card_controller_2 _output_get))
  (set `self.GroundAreas` _sorted_by_distance)
  ;[1 1 1] Get player characters in level
  (bind _arrayofaliveenemies (`/Game/Zomboat/Core/CombatEncounter/CardUI/BP_CardController.FindAlivePlayerCharactersInLevel` (`self.CastCardController`)))
  (set `self.PlayerCharacterActorsInLevel` _arrayofaliveenemies)
  ;[1 1 1] Store ref to HUD widget
  (bind _asw_player_hudwidget (cast `/Game/Zomboat/Core/CombatEncounter/3DWorld/W_PlayerHUDWidget` (`WidgetComponent.GetUserWidgetObject` (`self.HUDWidget`)))
    (:`then`
      _)
    (:`CastFailed`
      _))
  (set `self.HUDWidgetRef` _asw_player_hudwidget)
  (set `SkeletalMeshComponent.SkeletalMeshAsset` _characterinfo_skeletalmesh _mesh)
  (`SkeletalMeshComponent.SetAnimInstanceClass` _mesh _characterinfo_animationblueprint)
  (bind _output_get_2 (set `self.MaxStamina` _characterinfo_maxstamina))
  (set `self.CurrentStamina` _output_get_2)
  (`self.AttachEquipmentToCharacter`))

(event `self.ReceiveActorBeginOverlap`
  (params (OtherActor :type "Actor Object Reference"))
  (bind _asground_area (cast `/Game/Zomboat/Core/CombatEncounter/3DWorld/GroundArea` OtherActor))
  (bind _output_get (set `self.CurrentGroundArea` _asground_area))
  (if (or (`/Game/Zomboat/Core/CombatEncounter/3DWorld/GroundArea.IsDamageArea` _output_get) (`/Game/Zomboat/Core/CombatEncounter/3DWorld/GroundArea.IsCombatArea` _output_get))
    (set `self.CharInCombat?` true)))

(event `self.ReceiveTick`
  (params (DeltaSeconds :type "Float (single-precision)"))
  (if (<= (`self.CurrentHealth`) 0.0)
    ;[1 1 1] Handle player character death
    (bind _asbp_card_controller (cast `/Game/Zomboat/Core/CombatEncounter/CardUI/BP_CardController` (`GameplayStatics.GetPlayerController` 0)))
    (`/Game/Zomboat/Core/CombatEncounter/CardUI/BP_CardController.PlayerCharacterIsDying` _asbp_card_controller)
    (set `self.IsDying` true)
    (set `self.IsDead` true)))

(event `IsAttackingAnimTrigger`
  (set `self.IsAttacking` true)
  (`KismetSystemLibrary.Delay` 0.2)
  (set `self.IsAttacking` false))

(event `IsBlockingAnimTrigger`
  (set `self.IsBlocking` true)
  (`KismetSystemLibrary.Delay` 0.2)
  (set `self.IsBlocking` false))

(event `IsThrowingAnimTrigger`
  (set `self.IsThrowing` true)
  (`KismetSystemLibrary.Delay` 0.2)
  (set `self.IsThrowing` false))

(event `TakeDamage`
  (params (DamageToTake :type "Float (double-precision)"))
  (`self.Take Damage Func` DamageToTake)
  (set `self.IsTakingDamage` true)
  (`KismetSystemLibrary.Delay` 0.2)
  (set `self.IsTakingDamage` false))

(event `ModifyBlock`
  (params (BlockAmount :type "Float (double-precision)"))
  (`self.Modify Block Func` BlockAmount))

(event `Modify Stamina`
  (params (StaminaAmount :type "Float (double-precision)"))
  (`self.Modify Stamina Func` StaminaAmount))

(fn `AttachEquipmentToCharacter`
  (locals (LocalSlotIndex :type Integer) (LocalSocketName :type Name))
  (for (_array_element _array_index) (`.CharacterEquipment_48_41508C8F4C92115C21A36681661C9FB3` (break `/Game/Zomboat/Core/CombatEncounter/3DWorld/S_Characters` (`self.CharacterInfo`)))
    (set `local.LocalSlotIndex` _array_index)
    (bind _item (break `/Game/Zomboat/Core/BoatMap/EquipMenu/S_Slots` _array_element))
    (if (!= (`.RowName` (break `DataTableRowHandle` _item)) "NoItem")
      (bind _returnvalue (`|GetDataTableRow` (break `DataTableRowHandle` _item) (`.RowName` (break `DataTableRowHandle` _item)))
        (:`then`
          (bind _returnvalue_2 (`|SpawnActorFromClass` (`.ActorClass_33_BF4E304C44E64C56BD8747B526B139D8` (break `/Game/Zomboat/Core/CombatEncounter/CardUI/S_Items` _returnvalue)) (`KismetMathLibrary.MakeTransform` (0.0 0.0 0.0)) "Undefined" "MultiplyWithRoot" null null))
          (switch `int` (`local.LocalSlotIndex`)
            (:`0`
              (set `local.LocalSocketName` "HeadArmour"))
            (:`1`
              (set `local.LocalSocketName` "ArmRight"))
            (:`2`
              (set `local.LocalSocketName` "ArmLeft"))
            (:`3`
              (set `local.LocalSocketName` "WeaponRight"))
            (:`4`
              (set `local.LocalSocketName` "WeaponLeft")))
          (`self.K2_AttachToComponent` _returnvalue_2 (`self.Mesh`) (`local.LocalSocketName`) "SnapToTarget" "SnapToTarget" "SnapToTarget" true))))))

(fn `GetTutorialCharDetails`
  (bind _mesh (`self.Mesh`))
  (bind _mesh_2 (`self.Mesh`))
  (bind _mesh_3 (`self.Mesh`))
  (bind _asbp_game_instance (cast `/Game/Zomboat/Core/CombatEncounter/3DWorld/BP_GameInstance` (`GameplayStatics.GetGameInstance`)))
  (switch `/Game/Zomboat/Core/Tutorial/E_TutorialChars` (`self.IsTutorialCharacter`)
    (:`NewEnumerator0`
      (return))
    (:`NewEnumerator1`
      (bind (_tutorialcharacterone_charactername _tutorialcharacterone_skeletalmesh _tutorialcharacterone_animationblueprint _tutorialcharacterone_currenthealth _tutorialcharacterone_currentstamina _tutorialcharacterone_righthanditem _tutorialcharacterone_lefthanditem _tutorialcharacterone_headitem _tutorialcharacterone_bodyitem _tutorialcharacterone_armsitem _tutorialcharacterone_legsitem _tutorialcharacterone_maxhealth _tutorialcharacterone_maxstamina _tutorialcharacterone_characternumber _tutorialcharacterone_characterequipment) (break `/Game/Zomboat/Core/CombatEncounter/3DWorld/S_Characters` (`/Game/Zomboat/Core/CombatEncounter/3DWorld/BP_GameInstance.TutorialCharacterOne` _asbp_game_instance)))
      (bind _output_get (set `self.CharacterInfo` (make `/Game/Zomboat/Core/CombatEncounter/3DWorld/S_Characters` _tutorialcharacterone_charactername _tutorialcharacterone_skeletalmesh _tutorialcharacterone_animationblueprint _tutorialcharacterone_currenthealth _tutorialcharacterone_currentstamina "NewEnumerator0" "NewEnumerator0" "NewEnumerator0" "NewEnumerator0" "NewEnumerator0" "NewEnumerator0" _tutorialcharacterone_maxhealth _tutorialcharacterone_maxstamina _tutorialcharacterone_characternumber _tutorialcharacterone_characterequipment)))
      (set `SkeletalMeshComponent.SkeletalMeshAsset` (`.SkeletalMesh_6_F740C3C74A2A6B8E818ECF99C5ADAC90` (break `/Game/Zomboat/Core/CombatEncounter/3DWorld/S_Characters` _output_get)) _mesh_3)
      (`SkeletalMeshComponent.SetAnimInstanceClass` _mesh_3 (`.AnimationBlueprint_44_03747F9E47800859479062BC15C3BE9D` (break `/Game/Zomboat/Core/CombatEncounter/3DWorld/S_Characters` _output_get))))
    (:`NewEnumerator2`
      (bind (_tutorialcharactertwo_charactername _tutorialcharactertwo_skeletalmesh _tutorialcharactertwo_animationblueprint _tutorialcharactertwo_currenthealth _tutorialcharactertwo_currentstamina _tutorialcharactertwo_righthanditem _tutorialcharactertwo_lefthanditem _tutorialcharactertwo_headitem _tutorialcharactertwo_bodyitem _tutorialcharactertwo_armsitem _tutorialcharactertwo_legsitem _tutorialcharactertwo_maxhealth _tutorialcharactertwo_maxstamina _tutorialcharactertwo_characternumber _tutorialcharactertwo_characterequipment) (break `/Game/Zomboat/Core/CombatEncounter/3DWorld/S_Characters` (`/Game/Zomboat/Core/CombatEncounter/3DWorld/BP_GameInstance.TutorialCharacterTwo` _asbp_game_instance)))
      (bind _output_get_2 (set `self.CharacterInfo` (make `/Game/Zomboat/Core/CombatEncounter/3DWorld/S_Characters` _tutorialcharactertwo_charactername _tutorialcharactertwo_skeletalmesh _tutorialcharactertwo_animationblueprint _tutorialcharactertwo_currenthealth _tutorialcharactertwo_currentstamina "NewEnumerator0" "NewEnumerator0" "NewEnumerator0" "NewEnumerator0" "NewEnumerator0" "NewEnumerator0" _tutorialcharactertwo_maxhealth _tutorialcharactertwo_maxstamina _tutorialcharactertwo_characternumber _tutorialcharactertwo_characterequipment)))
      (set `SkeletalMeshComponent.SkeletalMeshAsset` (`.SkeletalMesh_6_F740C3C74A2A6B8E818ECF99C5ADAC90` (break `/Game/Zomboat/Core/CombatEncounter/3DWorld/S_Characters` _output_get_2)) _mesh_2)
      (`SkeletalMeshComponent.SetAnimInstanceClass` _mesh_2 (`.AnimationBlueprint_44_03747F9E47800859479062BC15C3BE9D` (break `/Game/Zomboat/Core/CombatEncounter/3DWorld/S_Characters` _output_get_2))))
    (:`NewEnumerator3`
      (bind (_tutorialcharacterthree_charactername _tutorialcharacterthree_skeletalmesh _tutorialcharacterthree_animationblueprint _tutorialcharacterthree_currenthealth _tutorialcharacterthree_currentstamina _tutorialcharacterthree_righthanditem _tutorialcharacterthree_lefthanditem _tutorialcharacterthree_headitem _tutorialcharacterthree_bodyitem _tutorialcharacterthree_armsitem _tutorialcharacterthree_legsitem _tutorialcharacterthree_maxhealth _tutorialcharacterthree_maxstamina _tutorialcharacterthree_characternumber _tutorialcharacterthree_characterequipment) (break `/Game/Zomboat/Core/CombatEncounter/3DWorld/S_Characters` (`/Game/Zomboat/Core/CombatEncounter/3DWorld/BP_GameInstance.TutorialCharacterThree` _asbp_game_instance)))
      (bind _output_get_3 (set `self.CharacterInfo` (make `/Game/Zomboat/Core/CombatEncounter/3DWorld/S_Characters` _tutorialcharacterthree_charactername _tutorialcharacterthree_skeletalmesh _tutorialcharacterthree_animationblueprint _tutorialcharacterthree_currenthealth _tutorialcharacterthree_currentstamina "NewEnumerator0" "NewEnumerator0" "NewEnumerator0" "NewEnumerator0" "NewEnumerator0" "NewEnumerator0" _tutorialcharacterthree_maxhealth _tutorialcharacterthree_maxstamina _tutorialcharacterthree_characternumber _tutorialcharacterthree_characterequipment)))
      (set `SkeletalMeshComponent.SkeletalMeshAsset` (`.SkeletalMesh_6_F740C3C74A2A6B8E818ECF99C5ADAC90` (break `/Game/Zomboat/Core/CombatEncounter/3DWorld/S_Characters` _output_get_3)) _mesh)
      (`SkeletalMeshComponent.SetAnimInstanceClass` _mesh (`.AnimationBlueprint_44_03747F9E47800859479062BC15C3BE9D` (break `/Game/Zomboat/Core/CombatEncounter/3DWorld/S_Characters` _output_get_3))))))

(fn `Modify Block Func`
  (params (Block :type "Float (double-precision)"))
  (bind _currentblock (`self.CurrentBlock`))
  (bind _mainhudwidget (`/Game/Zomboat/Core/CombatEncounter/CardUI/BP_CardController.MainHUDWidget` (`self.CastCardController`)))
  (bind _output_get (set `self.CurrentBlock` (+ (`self.CurrentBlock`) Block)))
  (set `TextBlock.Text` (`KismetTextLibrary.Conv_DoubleToText` _output_get "HalfToEven") (`/Game/Zomboat/Core/CombatEncounter/CardUI/W_CardHUD.BlockAmount` (`self.LinkedCardHUD`)))
  (switch `/Game/Zomboat/Core/CombatEncounter/3DWorld/E_CharacterNumbers` (`.CharacterNumber_36_DEC2414C4DB86685A278DFA85CADF1F7` (break `/Game/Zomboat/Core/CombatEncounter/3DWorld/S_Characters` (`self.CharacterInfo`)))
    (:`NewEnumerator0`
      (set `/Game/Zomboat/Core/CombatEncounter/CardUI/W_MainHUD.CharacterOneBlock` _currentblock _mainhudwidget))
    (:`NewEnumerator1`
      (set `/Game/Zomboat/Core/CombatEncounter/CardUI/W_MainHUD.CharacterTwoBlock` _currentblock _mainhudwidget))
    (:`NewEnumerator2`
      (set `/Game/Zomboat/Core/CombatEncounter/CardUI/W_MainHUD.CharacterThreeBlock` _currentblock _mainhudwidget))))

(fn `Modify Stamina Func`
  (params (StaminaAmount :type "Float (double-precision)"))
  (bind _currentstamina (`self.CurrentStamina`))
  (bind _mainhudwidget (`/Game/Zomboat/Core/CombatEncounter/CardUI/BP_CardController.MainHUDWidget` (`self.CastCardController`)))
  (bind _output_get (set `self.CurrentStamina` (+ (`self.CurrentStamina`) StaminaAmount)))
  (set `/Game/Zomboat/Core/CombatEncounter/CardUI/W_CardHUD.Stamina` _output_get (`self.LinkedCardHUD`))
  (switch `/Game/Zomboat/Core/CombatEncounter/3DWorld/E_CharacterNumbers` (`.CharacterNumber_36_DEC2414C4DB86685A278DFA85CADF1F7` (break `/Game/Zomboat/Core/CombatEncounter/3DWorld/S_Characters` (`self.CharacterInfo`)))
    (:`NewEnumerator0`
      (set `/Game/Zomboat/Core/CombatEncounter/CardUI/W_MainHUD.CharacterOneStamina` _currentstamina _mainhudwidget))
    (:`NewEnumerator1`
      (set `/Game/Zomboat/Core/CombatEncounter/CardUI/W_MainHUD.CharacterTwoStamina` _currentstamina _mainhudwidget))
    (:`NewEnumerator2`
      (set `/Game/Zomboat/Core/CombatEncounter/CardUI/W_MainHUD.CharacterThreeStamina` _currentstamina _mainhudwidget))))

(fn `ResetStamina`
  (bind _output_get (set `self.CurrentStamina` (`self.MaxStamina`)))
  (set `/Game/Zomboat/Core/CombatEncounter/CardUI/W_CardHUD.Stamina` _output_get (`self.LinkedCardHUD`))
  (switch `/Game/Zomboat/Core/CombatEncounter/3DWorld/E_CharacterNumbers` (`.CharacterNumber_36_DEC2414C4DB86685A278DFA85CADF1F7` (break `/Game/Zomboat/Core/CombatEncounter/3DWorld/S_Characters` (`self.CharacterInfo`)))))

(fn `Take Damage Func`
  (params (DamageToTake :type "Float (double-precision)"))
  (bind _currenthealth (`self.CurrentHealth`))
  (bind _returnvalue (- (`self.CurrentBlock`) DamageToTake))
  (bind _mainhudwidget (`/Game/Zomboat/Core/CombatEncounter/CardUI/BP_CardController.MainHUDWidget` (`self.CastCardController`)))
  (set `self.AttackDamageAfterBlock` (- DamageToTake (`self.CurrentBlock`)))
  (if (>= _returnvalue 0.0)
    (bind _output_get (set `self.CurrentBlock` _returnvalue))
    ;[1 1 1] Update Character HUD
    (set `TextBlock.Text` (`KismetTextLibrary.Conv_DoubleToText` _output_get "HalfToEven") (`/Game/Zomboat/Core/CombatEncounter/CardUI/W_CardHUD.BlockAmount` (`self.LinkedCardHUD`)))
    (`self.UpdateMainHUDBlock` 0.0)
    (else
      (bind _output_get_2 (set `self.CurrentBlock` 0.0))
      ;[1 1 1] Update Character HUD
      (set `TextBlock.Text` (`KismetTextLibrary.Conv_DoubleToText` _output_get_2 "HalfToEven") (`/Game/Zomboat/Core/CombatEncounter/CardUI/W_CardHUD.BlockAmount` (`self.LinkedCardHUD`)))
      (`self.UpdateMainHUDBlock` (`self.CurrentBlock`))
      (bind _output_get_3 (set `self.CurrentHealth` (- (`self.CurrentHealth`) (`self.AttackDamageAfterBlock`))))
      (set `/Game/Zomboat/Core/CombatEncounter/CardUI/W_CardHUD.Health` _output_get_3 (`self.LinkedCardHUD`))
      (switch `/Game/Zomboat/Core/CombatEncounter/3DWorld/E_CharacterNumbers` (`.CharacterNumber_36_DEC2414C4DB86685A278DFA85CADF1F7` (break `/Game/Zomboat/Core/CombatEncounter/3DWorld/S_Characters` (`self.CharacterInfo`)))
        (:`NewEnumerator0`
          (set `/Game/Zomboat/Core/CombatEncounter/CardUI/W_MainHUD.CharacterOneHealth` _currenthealth _mainhudwidget))
        (:`NewEnumerator1`
          (set `/Game/Zomboat/Core/CombatEncounter/CardUI/W_MainHUD.CharacterTwoHealth` _currenthealth _mainhudwidget))
        (:`NewEnumerator2`
          (set `/Game/Zomboat/Core/CombatEncounter/CardUI/W_MainHUD.CharacterThreeHealth` _currenthealth _mainhudwidget))))))

(fn `UpdateCharacterDetailsInGameInstance`
  (locals (LocalCastGameInstance :type "/Game/Zomboat/Core/CombatEncounter/3DWorld/BP_GameInstance Object Reference"))
  (bind (_characterinfo_charactername _characterinfo_skeletalmesh _characterinfo_animationblueprint _characterinfo_currenthealth _characterinfo_currentstamina _characterinfo_righthanditem _characterinfo_lefthanditem _characterinfo_headitem _characterinfo_bodyitem _characterinfo_armsitem _characterinfo_legsitem _characterinfo_maxhealth _characterinfo_maxstamina _characterinfo_characternumber _characterinfo_characterequipment) (break `/Game/Zomboat/Core/CombatEncounter/3DWorld/S_Characters` (`self.CharacterInfo`)))
  (bind _s_characters (make `/Game/Zomboat/Core/CombatEncounter/3DWorld/S_Characters` _characterinfo_charactername _characterinfo_skeletalmesh _characterinfo_animationblueprint (`self.CurrentHealth`) _characterinfo_currentstamina "NewEnumerator0" "NewEnumerator0" "NewEnumerator0" "NewEnumerator0" "NewEnumerator0" "NewEnumerator0" _characterinfo_maxhealth _characterinfo_maxstamina _characterinfo_characternumber _characterinfo_characterequipment))
  (bind _asbp_game_instance (cast `/Game/Zomboat/Core/CombatEncounter/3DWorld/BP_GameInstance` (`GameplayStatics.GetGameInstance`)))
  (set `local.LocalCastGameInstance` _asbp_game_instance)
  (switch `/Game/Zomboat/Core/CombatEncounter/3DWorld/E_CharacterNumbers` _characterinfo_characternumber
    (:`NewEnumerator0`
      (set `/Game/Zomboat/Core/CombatEncounter/3DWorld/BP_GameInstance.PlayerCharacterOne` _s_characters (`local.LocalCastGameInstance`)))
    (:`NewEnumerator1`
      (set `/Game/Zomboat/Core/CombatEncounter/3DWorld/BP_GameInstance.PlayerCharacterTwo` _s_characters (`local.LocalCastGameInstance`)))
    (:`NewEnumerator2`
      (set `/Game/Zomboat/Core/CombatEncounter/3DWorld/BP_GameInstance.PlayerCharacterThree` _s_characters (`local.LocalCastGameInstance`)))))

(fn `UpdateMainHUDBlock`
  (params (CurrentBlock :type "Float (double-precision)"))
  (locals (LocalCurrentBlock :type "Float (double-precision)"))
  (bind _localcurrentblock (`local.LocalCurrentBlock`))
  (bind _mainhudwidget (`/Game/Zomboat/Core/CombatEncounter/CardUI/BP_CardController.MainHUDWidget` (`self.CastCardController`)))
  (set `local.LocalCurrentBlock` CurrentBlock)
  (switch `/Game/Zomboat/Core/CombatEncounter/3DWorld/E_CharacterNumbers` (`.CharacterNumber_36_DEC2414C4DB86685A278DFA85CADF1F7` (break `/Game/Zomboat/Core/CombatEncounter/3DWorld/S_Characters` (`self.CharacterInfo`)))
    (:`NewEnumerator0`
      (set `/Game/Zomboat/Core/CombatEncounter/CardUI/W_MainHUD.CharacterOneBlock` _localcurrentblock _mainhudwidget))
    (:`NewEnumerator1`
      (set `/Game/Zomboat/Core/CombatEncounter/CardUI/W_MainHUD.CharacterTwoBlock` _localcurrentblock _mainhudwidget))
    (:`NewEnumerator2`
      (set `/Game/Zomboat/Core/CombatEncounter/CardUI/W_MainHUD.CharacterThreeBlock` _localcurrentblock _mainhudwidget))))

(fn `UserConstructionScript`)