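; Placed spawner actor for the combat encounter world that creates one of the three player characters at its own transform.
; On BeginPlay it reads the ActorToSpawn selector and fetches the matching character record from BP_GameInstance.
; SpawnCharacter then spawns a BP_PlayerCharacter, passing that record's name, mesh, health, stamina and equipped items as spawn parameters.
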(event `self.ReceiveBeginPlay`
  (`self.SpawnActor`))

(event `SpawnActor`
  (bind _asbp_game_instance (cast `/Game/Zomboat/Core/CombatEncounter/3DWorld/BP_GameInstance` (`GameplayStatics.GetGameInstance`)))
  (switch `/Game/Zomboat/Core/CombatEncounter/3DWorld/E_CharacterNumbers` (`self.ActorToSpawn`)
    (:`NewEnumerator0`
      (`self.Spawn Character` (`/Game/Zomboat/Core/CombatEncounter/3DWorld/BP_GameInstance.PlayerCharacterOne` _asbp_game_instance)))
    (:`NewEnumerator1`
      (`self.Spawn Character` (`/Game/Zomboat/Core/CombatEncounter/3DWorld/BP_GameInstance.PlayerCharacterTwo` _asbp_game_instance)))
    (:`NewEnumerator2`
      (`self.Spawn Character` (`/Game/Zomboat/Core/CombatEncounter/3DWorld/BP_GameInstance.PlayerCharacterThree` _asbp_game_instance)))))

(fn `Spawn Character`
  (params (CharacterInfo :type "/Game/Zomboat/Core/CombatEncounter/3DWorld/S_Characters Structure (by ref)"))
  (bind (_charactername _skeletalmesh _currenthealth _currentstamina _righthanditem _lefthanditem _headitem _bodyitem _armsitem _legsitem _maxhealth _maxstamina _characternumber) (break `/Game/Zomboat/Core/CombatEncounter/3DWorld/S_Characters` CharacterInfo))
  (`|SpawnActorFromClass` "/Game/Zomboat/Core/CombatEncounter/3DWorld/BP_PlayerCharacter.BP_PlayerCharacter_C" (`self.GetTransform`) "Undefined" "MultiplyWithRoot" null false _currentstamina _currenthealth "NewEnumerator0" "NewEnumerator0" "NewEnumerator0" "NewEnumerator0" "NewEnumerator0" "NewEnumerator0" (make `/Game/Zomboat/Core/CombatEncounter/3DWorld/S_Characters` _charactername _skeletalmesh _currenthealth _currentstamina _righthanditem _lefthanditem _headitem _bodyitem _armsitem _legsitem _maxhealth _maxstamina _characternumber) null))

(fn `UserConstructionScript`)