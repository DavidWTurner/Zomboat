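; BP_GroundItem is a world pickup actor for the 3D combat encounter, representing one item type chosen by an enum.
; On BeginPlay it looks up that type's row in DT_GroundItems, stores its name, display name, linked cards and mesh, and applies the mesh.
; When its mesh overlaps an actor tagged GroundArea, it records that GroundArea as its current area.
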(event `self.ReceiveBeginPlay`
  (bind _returnvalue (`|GetDataTableRow` "/Game/Zomboat/Core/CombatEncounter/CardUI/DT_GroundItems.DT_GroundItems" (`KismetStringLibrary.Conv_StringToName` (`|GetEnumeratorNameAsString` (`self.GroundItemToBe`))))
    (:`then`
      (bind _output_get (set `self.GroundItemInfo` (make `/Game/Zomboat/Core/CombatEncounter/CardUI/S_GroundItems` (break `/Game/Zomboat/Core/CombatEncounter/CardUI/S_GroundItems` _returnvalue) (`.DisplayName_9_A67224244A7E7734D4E604954FDB85EA` (break `/Game/Zomboat/Core/CombatEncounter/CardUI/S_GroundItems` _returnvalue)) (`.LinkedCards_6_C1A629F0419CFE7A32BEC09201B617F7` (break `/Game/Zomboat/Core/CombatEncounter/CardUI/S_GroundItems` _returnvalue)) (`.StaticMesh_13_4946CA9E44AA1DDBD3266CB8A4F94F10` (break `/Game/Zomboat/Core/CombatEncounter/CardUI/S_GroundItems` _returnvalue)))))
      (`StaticMeshComponent.SetStaticMesh` (`self.StaticMesh`) (`.StaticMesh_13_4946CA9E44AA1DDBD3266CB8A4F94F10` (break `/Game/Zomboat/Core/CombatEncounter/CardUI/S_GroundItems` _output_get))))))

(event `self.StaticMesh.OnComponentBeginOverlap`
  (params (OverlappedComponent :type "PrimitiveComponent Object Reference") (OtherActor :type "Actor Object Reference") (OtherComp :type "PrimitiveComponent Object Reference") (OtherBodyIndex :type Integer) (bFromSweep :type Boolean) (SweepResult :type "HitResult Structure (by ref)"))
  (if (`self.ActorHasTag` OtherActor "GroundArea")
    (bind _asground_area (cast `/Game/Zomboat/Core/CombatEncounter/3DWorld/GroundArea` OtherActor))
    (set `self.CurrentGroundArea` _asground_area)))

(fn `UserConstructionScript`)