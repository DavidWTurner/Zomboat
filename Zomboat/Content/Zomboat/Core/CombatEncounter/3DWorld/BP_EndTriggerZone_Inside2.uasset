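; BP_EndTriggerZone_Inside2 is a trigger zone that ends a combat encounter once all enemies are gone.
; When an actor tagged PlayerCharacter overlaps its Box, it checks that no BP_EnemyCharacter actors remain in the level.
; If none remain, every BP_PlayerCharacter updates its character details in the game instance, then the RewardsScreen_BP2 widget is created and added to the viewport.
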(event `self.ReceiveBeginPlay`)

(event `self.Box.OnComponentBeginOverlap`
  (params (OverlappedComponent :type "PrimitiveComponent Object Reference") (OtherActor :type "Actor Object Reference") (OtherComp :type "PrimitiveComponent Object Reference") (OtherBodyIndex :type Integer) (bFromSweep :type Boolean) (SweepResult :type "HitResult Structure (by ref)"))
  (if (`self.ActorHasTag` OtherActor "PlayerCharacter")
    (bind _outactors (`GameplayStatics.GetAllActorsOfClass` "/Game/Zomboat/Core/CombatEncounter/3DWorld/BP_EnemyCharacter.BP_EnemyCharacter_C"))
    (if (== (`KismetArrayLibrary.Array_Length` _outactors) 0)
      (bind _outactors_2 (`GameplayStatics.GetAllActorsOfClass` "/Game/Zomboat/Core/CombatEncounter/3DWorld/BP_PlayerCharacter.BP_PlayerCharacter_C"))
      (bind _output_get (set `self.PlayerCharactersInLevel` _outactors_2))
      (for _array_element _output_get
        (`/Game/Zomboat/Core/CombatEncounter/3DWorld/BP_PlayerCharacter.UpdateCharacterDetailsInGameInstance` _array_element))
      (bind _returnvalue (`|CreateWidget` "/Game/Zomboat/Developers/Phil/RewardsScreen_BP2.RewardsScreen_BP2_C"))
      (`UserWidget.AddToViewport` _returnvalue 0))))

(fn `UserConstructionScript`)