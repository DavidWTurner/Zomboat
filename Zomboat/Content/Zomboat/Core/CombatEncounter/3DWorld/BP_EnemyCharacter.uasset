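; Zombie enemy for turn-based combat that advances along GroundArea zones and attacks player characters.
; On spawn it sorts zones by distance from player spawn and walks to its starting one; overlaps set the next zone toward players.
; Each turn in combat executes the intent, then picks and displays the next: random-target, random-damage attack if in range, otherwise move.
; Damage updates the HUD; Tick handles death, clearing players' combat flags when no enemy is near.
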(event `self.ReceiveBeginPlay`
  (bind _outactors (`GameplayStatics.GetAllActorsOfClass` "/Game/Zomboat/Core/CombatEncounter/3DWorld/BP_PlayerCharacter.BP_PlayerCharacter_C"))
  (set `self.PlayerCharactersInLevel` _outactors)
  (bind _outactors_2 (`GameplayStatics.GetAllActorsOfClass` "BP_EnemyCharacter_C"))
  (set `self.EnemyCharactersInLevel` _outactors_2)
  (bind _asai_enemy_hudwidget (cast `/Game/Zomboat/Core/CombatEncounter/3DWorld/AI_EnemyHUDWidget` (`WidgetComponent.GetUserWidgetObject` (`self.HUDWidget`))))
  (set `self.HUDWidgetREF` _asai_enemy_hudwidget)
  (set `self.CurrentHealth` (`self.MaxHealth`))
  (`KismetSystemLibrary.Delay` 1.0)
  (bind _outactors_3 (`GameplayStatics.GetAllActorsOfClass` "/Game/Zomboat/Core/CombatEncounter/3DWorld/GroundArea.GroundArea_C"))
  (bind _output_get (set `self.GroundAreas` _outactors_3))
  (bind _asbp_card_controller (cast `/Game/Zomboat/Core/CombatEncounter/CardUI/BP_CardController` (`GameplayStatics.GetPlayerController` 0)))
  (bind _sorted_by_distance (`/Game/Zomboat/Core/CombatEncounter/CardUI/BP_CardController.SortArraybyDistanceFromPlayerSpawn` _asbp_card_controller _output_get))
  (bind _output_get_2 (set `self.GroundAreas` _sorted_by_distance))
  (for _array_element _output_get_2
    (if (== (`/Game/Zomboat/Core/CombatEncounter/3DWorld/GroundArea.PositionInArray` _array_element) (`self.StartingGroundAreaNum`))
      (bind _returnvalue (`self.GetTransform` _array_element))
      (`AITask_MoveTo.AIMoveTo` (`AIBlueprintHelperLibrary.GetAIController` self) (`KismetMathLibrary.MakeVector` (+ (.x (.location _returnvalue)) (`KismetMathLibrary.RandomFloatInRange` -250.0 250.0)) (+ (.y (.location _returnvalue)) (`KismetMathLibrary.RandomFloatInRange` -200.0 200.0)) (.z (.location _returnvalue))) null))))

(event `self.ReceiveActorBeginOverlap`
  (params (OtherActor :type "Actor Object Reference"))
  (bind _groundareas (`self.GroundAreas`))
  ;[1 1 1] When entering a ground area, mark the next ground area as the next to move to
  (bind _asground_area (cast `/Game/Zomboat/Core/CombatEncounter/3DWorld/GroundArea` OtherActor))
  (set `self.CurrentGroundArea` _asground_area)
  (set `self.GroundAreaToMoveTo` (`|GetArrayItem` _groundareas (- (`KismetArrayLibrary.Array_Find` _groundareas (`self.CurrentGroundArea`)) 1))))

(event `self.ReceiveTick`
  (params (DeltaSeconds :type "Float (single-precision)"))
  (if (<= (`self.CurrentHealth`) 0.0)
    ;[1 1 1] Attempt at removing players from combat, will most likely remove
    (bind _outactors (`GameplayStatics.GetAllActorsOfClass` "BP_EnemyCharacter_C"))
    (bind _output_get (set `self.EnemyCharactersInLevel` _outactors))
    (if (> (`GameplayStatics.FindNearestActor` (`self.K2_GetActorLocation`) _output_get) 900.0)
      (for _array_element (`self.PlayerCharactersInLevel`)
        (set `/Game/Zomboat/Core/CombatEncounter/3DWorld/BP_PlayerCharacter.CharInCombat?` false _array_element)))
    (`self.K2_DestroyActor`)))

(event `EnemyTurn_Event`
  (bind (_returnvalue_x _returnvalue_y _returnvalue_z) (`KismetMathLibrary.BreakVector` (`self.K2_GetActorLocation` (`self.GroundAreaToMoveTo`))))
  ;[1 1 1] Small delay to make the enemy turns not instant
  (`KismetSystemLibrary.Delay` 0.5)
  (if (`self.InCombat`)
    (`KismetSystemLibrary.PrintString` "our turn now")
    (switch `/Game/Zomboat/Core/CombatEncounter/3DWorld/E_EnemyIntents` (`self.CurrentIntent`)
      (:`NewEnumerator0`
        (`/Game/Zomboat/Core/CombatEncounter/3DWorld/BP_PlayerCharacter.TakeDamage` (`self.AttackTarget`) (`KismetMathLibrary.Conv_IntToDouble` (`self.AttackDamageThisAttack`))))
      (:`NewEnumerator2`
        (`KismetSystemLibrary.PrintString` "zom shuffe?")
        (`AITask_MoveTo.AIMoveTo` (`AIBlueprintHelperLibrary.GetAIController` self) (`KismetMathLibrary.MakeVector` (+ _returnvalue_x (`KismetMathLibrary.RandomFloatInRange` -400.0 400.0)) (+ _returnvalue_y (`KismetMathLibrary.RandomFloatInRange` -200.0 200.0)) _returnvalue_z) null
          (:`OnMoveFinished`
            _)))
      (:`NewEnumerator3`
        _))
    (`self.EnemyAttackAndIntent`)))

(event `TakeDamage_Event`
  (params (DamageToTake :type "Float (double-precision)"))
  (`KismetSystemLibrary.PrintString` "Damage event?")
  (bind _output_get (set `self.CurrentHealth` (- (`self.CurrentHealth`) DamageToTake)))
  (set `/Game/Zomboat/Core/CombatEncounter/3DWorld/AI_EnemyHUDWidget.Health` _output_get (`self.HUDWidgetREF`)))

(fn `EnemyAttackAndIntent`
  (locals (PlayerInRange :type Boolean) (PlayersInRange :type "Array of /Game/Zomboat/Core/CombatEncounter/3DWorld/BP_PlayerCharacter Object Reference"))
  (bind _groundareas (`self.GroundAreas`))
  (set `local.PlayerInRange` false)
  (`KismetArrayLibrary.Array_Clear` (`local.PlayersInRange`))
  (for _array_element (`self.PlayerCharactersInLevel`)
    (bind _returnvalue (<= (- (`KismetArrayLibrary.Array_Find` _groundareas (`self.CurrentGroundArea`)) (`KismetArrayLibrary.Array_Find` _groundareas (`/Game/Zomboat/Core/CombatEncounter/3DWorld/BP_PlayerCharacter.CurrentGroundArea` _array_element))) (`self.EnemyAttackRange`)))
    (if _returnvalue
      (set `local.PlayerInRange` _returnvalue)
      (`KismetArrayLibrary.Array_Add` (`local.PlayersInRange`) _array_element)))
  (if (`local.PlayerInRange`)
    (set `self.CurrentIntent` "NewEnumerator0")
    ;[1 1 1] Randomise damage
    (set `self.AttackDamageThisAttack` (`KismetMathLibrary.RandomIntegerInRange` (`self.MinAttackDamage`) (`self.MaxAttackDamage`)))
    ;[1 1 1] Random Target
    (bind _output_get (set `self.AttackTarget` (`KismetArrayLibrary.Array_Random` (`local.PlayersInRange`))))
    (bind _characterinfo_charactername (break `/Game/Zomboat/Core/CombatEncounter/3DWorld/S_Characters` (`/Game/Zomboat/Core/CombatEncounter/3DWorld/BP_PlayerCharacter.CharacterInfo` _output_get)))
    (set `TextBlock.Text` (`KismetTextLibrary.Conv_StringToText` (`KismetStringLibrary.Concat_StrStr` "Attacking " (`KismetTextLibrary.Conv_TextToString` _characterinfo_charactername) "For " (`KismetStringLibrary.Conv_IntToString` (`self.AttackDamageThisAttack`)) " Damage")) (`/Game/Zomboat/Core/CombatEncounter/3DWorld/AI_EnemyHUDWidget.EnemyIntent` (`self.HUDWidgetREF`)))
    (else
      (set `self.CurrentIntent` "NewEnumerator2")
      (`KismetSystemLibrary.PrintString` "Out of range, attempt to move")
      (set `TextBlock.Text` (`KismetTextLibrary.Conv_StringToText` "Moving Forward") (`/Game/Zomboat/Core/CombatEncounter/3DWorld/AI_EnemyHUDWidget.EnemyIntent` (`self.HUDWidgetREF`))))))

(fn `UserConstructionScript`)