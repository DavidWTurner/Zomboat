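; Player controller for the boat map that lets the player click crew characters to open their equipment menus.
; On BeginPlay it creates a hidden W_CharacterEquip widget for every BP_BoatCharacter, linked both ways, and enables the mouse cursor.
; Left-click traces for pawns, showing only the clicked character's widget, making a clicked cat meow, or hiding all widgets on a miss.
; A parallel UI_Inventory version of this logic is present but disconnected.
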(event `self.ReceiveBeginPlay`
  (bind _characterhud (`self.CharacterHUD`))
  (bind _outactors (`GameplayStatics.GetAllActorsOfClass` "/Game/Zomboat/Core/BoatMap/BP_BoatCharacter.BP_BoatCharacter_C"))
  (bind _output_get (set `self.BoatCharactersInLevel` _outactors))
  (for _array_element _output_get
    (bind _returnvalue (`|CreateWidget` "/Game/Zomboat/Core/BoatMap/EquipMenu/W_CharacterEquip.W_CharacterEquip_C" self _array_element))
    (set `/Game/Zomboat/Core/BoatMap/BP_BoatCharacter.LinkedEquipHUD` _returnvalue _array_element)
    (bind _output_get_2 (set `self.CharacterHUD` _returnvalue))
    (`KismetArrayLibrary.Array_Add` (`self.HUDWidgets`) _output_get_2)
    (`UserWidget.AddToViewport` _characterhud 0)
    (`WidgetBlueprintLibrary.SetInputMode_GameAndUIEx` self _characterhud "DoNotLock" false)
    (set `self.bShowMouseCursor` true)
    (`Widget.SetVisibility` (`self.CharacterHUD`) "Hidden")))

(event `Key|LeftMouseButton`
  (params (Key :type "Key Structure"))
  (bind _loopactor (`self.LoopActor`))
  (bind (_hitresult _returnvalue) (`self.GetHitResultUnderCursorForObjects` (`|MakeArray` "ObjectTypeQuery3" :!type "EObjectTypeQuery Enum")))
  (bind (_bblockinghit _binitialoverlap _time _distance _location _impactpoint _normal _impactnormal _physmat _hitactor) (`GameplayStatics.BreakHitResult` _hitresult))
  (:`Pressed`
    (if _returnvalue
      (if (`KismetSystemLibrary.IsValid` _hitactor)
        (if (`self.ActorHasTag` _hitactor "BoatCharacter")
          (set `self.ClickedActor` _hitactor)
          (for _array_element (`self.BoatCharactersInLevel`)
            (bind _output_get (set `self.LoopActor` _array_element))
            (if (`/Game/Zomboat/Core/BoatMap/BP_BoatCharacter.IsClicked` _output_get)
              (set `/Game/Zomboat/Core/BoatMap/BP_BoatCharacter.IsClicked` false _loopactor)
              (`Widget.SetVisibility` (`|GetArrayItem` (`self.HUDWidgets`) (`KismetArrayLibrary.Array_Find` (`self.BoatCharactersInLevel`) _loopactor)) "Hidden")))
          (bind _asbp_boat_character (cast `/Game/Zomboat/Core/BoatMap/BP_BoatCharacter` (`self.ClickedActor`)))
          (set `/Game/Zomboat/Core/BoatMap/BP_BoatCharacter.IsClicked` true _asbp_boat_character)
          (`Widget.SetVisibility` (`|GetArrayItem` (`self.HUDWidgets`) (`KismetArrayLibrary.Array_Find` (`self.BoatCharactersInLevel`) _asbp_boat_character)) "Visible")
          (elif (`self.ActorHasTag` _hitactor "Cat")
            (bind _ascat_bp (cast `/Game/Zomboat/Core/BoatMap/Cat_BP` _hitactor))
            (`/Game/Zomboat/Core/BoatMap/Cat_BP.Meow` _ascat_bp))))
      (else
        (for _array_element_2 (`self.HUDWidgets`)
          (`Widget.SetVisibility` _array_element_2 "Hidden"))))))

(event `Key|LeftMouseButton`
  (params (Key :type "Key Structure")))

(fn `UserConstructionScript`)