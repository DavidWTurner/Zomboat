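; BP_BoatCharacter is a character for the boat map that displays a looping animated mesh and holds an item inventory.
; On BeginPlay it applies the mesh from CharacterInfo and loops one animation in single-node mode.
; It then seeds PlayerSlots through AddItem with a zero-amount DT_Items row for every E_Items value, using enum names as row names.
; ShowInvUI toggles the inventory widget, cursor and input mode, but is marked as unused.
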(event `self.ReceiveBeginPlay`
  (bind _skeletalmesh (`self.SkeletalMesh`))
  (bind (_characterinfo_charactername _characterinfo_skeletalmesh) (break `/Game/Zomboat/Core/CombatEncounter/3DWorld/S_Characters` (`self.CharacterInfo`)))
  (bind _animation (`self.Animation`))
  (`SkeletalMeshComponent.SetSkeletalMeshAsset` (`self.SkeletalMesh`) _characterinfo_skeletalmesh)
  (`SkeletalMeshComponent.SetAnimationMode` _skeletalmesh "AnimationSingleNode" true)
  (`SkeletalMeshComponent.SetAnimation` _skeletalmesh _animation)
  (`SkeletalMeshComponent.PlayAnimation` _skeletalmesh _animation true)
  (bind _enumvalue (foreach `/Game/Zomboat/Core/CombatEncounter/CardUI/E_Items` true)
    (:`LoopBody`
      (`self.AddItem` (make `/Game/Zomboat/Core/BoatMap/EquipMenu/S_Slots` (make `DataTableRowHandle` "/Game/Zomboat/Core/CombatEncounter/CardUI/DT_Items.DT_Items" (`KismetStringLibrary.Conv_StringToName` (`|GetEnumeratorNameAsString` _enumvalue))))))))

(event `ShowInvUI`
  (bind _ui (`self.UI`))
  (bind _returnvalue (`Widget.GetOwningPlayer` _ui))
  ;[1 1 1] not in use currently
  (`/Engine/EditorBlueprintResources/StandardMacros.FlipFlop`
    (:`A`
      (bind _returnvalue_2 (`|CreateWidget` "/Game/Zomboat/Core/BoatMap/EquipMenu/UI_Inventory.UI_Inventory_C" null null))
      (set `self.UI` _returnvalue_2)
      (`UserWidget.AddToViewport` _ui 0)
      (set `PlayerController.bShowMouseCursor` true _returnvalue)
      (`WidgetBlueprintLibrary.SetInputMode_GameAndUIEx` null _ui))
    (:`B`
      (set `PlayerController.bShowMouseCursor` false _returnvalue)
      (`WidgetBlueprintLibrary.SetInputMode_GameOnly` _returnvalue)
      (`Widget.RemoveFromParent` (`self.UI`)))))

(fn `AddItem`
  (params (Item :type "/Game/Zomboat/Core/BoatMap/EquipMenu/S_Slots Structure"))
  (`KismetArrayLibrary.Array_Add` (`self.PlayerSlots`) Item))

(fn `UserConstructionScript`)