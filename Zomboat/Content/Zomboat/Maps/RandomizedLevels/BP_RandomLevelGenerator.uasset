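; Generates a random map at BeginPlay by filling a NumX by NumY grid, centered on the world origin, with streamed sublevels.
; Each cell picks randomly from the default level names, or from the first SpecificLevelInfo entry matching its one-based coordinates.
; Flagged entries get random coordinates beforehand, with no collision check.
; Sublevels are streaming-level instances named by cell, offset by LevelSize, unrotated and set to block on load.
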(event `self.ReceiveBeginPlay`
  (`self.CheckForEntriesThatNeedCoords`)
  (for _index (range (`self.NumX`))
    (set `self.LoopX` _index)
    (for _index_2 (range (`self.NumY`))
      (set `self.LoopY` _index_2)
      (bind (_leveldetails1 _foundinformation1) (`self.CheckForSpecificLevelInfo`))
      (if _foundinformation1
        (`self.PickAndSpawnLevelFromArray` (`.LevelNames_6_0B3DB06747A37C930A029A8570629656` (break `/Game/Zomboat/Maps/RandomizedLevels/S_SpecificLevelInfo` _leveldetails1)))
        (else
          (`self.PickAndSpawnLevelFromArray` (`self.LevelNames`)))))))

(fn `CheckForEntriesThatNeedCoords`
  (for (_array_element _array_index) (`self.SpecificLevelInfo`)
    (bind (_coordinates _levelnames _getrandomcoordsonplay) (break `/Game/Zomboat/Maps/RandomizedLevels/S_SpecificLevelInfo` _array_element))
    (if _getrandomcoordsonplay
      (`KismetArrayLibrary.Array_Set` (`self.SpecificLevelInfo`) _array_index (make `/Game/Zomboat/Maps/RandomizedLevels/S_SpecificLevelInfo` (`KismetMathLibrary.MakeVector` (`KismetMathLibrary.Conv_IntToDouble` (`KismetMathLibrary.RandomIntegerInRange` 1 (`self.NumX`))) (`KismetMathLibrary.Conv_IntToDouble` (`KismetMathLibrary.RandomIntegerInRange` 1 (`self.NumY`)))) _levelnames _getrandomcoordsonplay))))
  (return))

(fn `CheckForSpecificLevelInfo`
  (returns (LevelDetails1 :type "/Game/Zomboat/Maps/RandomizedLevels/S_SpecificLevelInfo Structure") (FoundInformation1 :type Boolean))
  (locals (LevelDetails :type "/Game/Zomboat/Maps/RandomizedLevels/S_SpecificLevelInfo Structure") (FoundInformation :type Boolean))
  (set `local.FoundInformation` false)
  (for _array_element (`self.SpecificLevelInfo`)
    (if (not (`local.FoundInformation`))
      (if (and (== (+ (`KismetMathLibrary.Round` (.x (`.Coordinates_2_655565434D9EB165A3760C9A1394DB36` (break `/Game/Zomboat/Maps/RandomizedLevels/S_SpecificLevelInfo` _array_element)))) -1) (`self.LoopX`)) (== (+ (`KismetMathLibrary.Round` (.y (`.Coordinates_2_655565434D9EB165A3760C9A1394DB36` (break `/Game/Zomboat/Maps/RandomizedLevels/S_SpecificLevelInfo` _array_element)))) -1) (`self.LoopY`)))
        (set `local.LevelDetails` _array_element)
        (set `local.FoundInformation` true))))
  (return (`local.LevelDetails`) (`local.FoundInformation`)))

(fn `PickAndSpawnLevelFromArray`
  (params (LevelNames :type "Array of Name"))
  (bind _returnvalue (`LevelStreaming.CreateInstance` (`GameplayStatics.GetStreamingLevel` (`|GetArrayItem` LevelNames (`KismetMathLibrary.RandomIntegerInRange` 0 (`KismetArrayLibrary.Array_LastIndex` LevelNames)))) (`KismetStringLibrary.Concat_StrStr` (`KismetStringLibrary.Conv_IntToString` (`self.LoopX`)) "x" (`KismetStringLibrary.Conv_IntToString` (`self.LoopY`)))))
  (set `LevelStreaming.LevelTransform` (`KismetMathLibrary.MakeTransform` (`KismetMathLibrary.MakeVector` (+ (- (* (`self.LoopX`) (`self.LevelSize`)) (/ (* (`self.NumX`) (`self.LevelSize`)) 2.0)) (/ (`self.LevelSize`) 2.0)) (+ (- (* (`self.LoopY`) (`self.LevelSize`)) (/ (* (`self.NumY`) (`self.LevelSize`)) 2.0)) (/ (`self.LevelSize`) 2.0)))) _returnvalue)
  (set `LevelStreaming.bShouldBlockOnLoad` true _returnvalue)
  (set `LevelStreaming.bShouldBeLoaded` true _returnvalue)
  (set `LevelStreaming.bShouldBeVisible` true _returnvalue))

(fn `UserConstructionScript`)